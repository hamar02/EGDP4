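; NPCPawn is a base 2D Paper flipbook NPC pawn with movement, facing, damage and death, leaving state and animation functions empty.
; Once activated, Tick calls UpdateState, applies swept X and Y offsets separately from Movement and MoveSpeed, and flips the flipbook by horizontal direction.
; Damage targets the attacker and lowers Health, either pausing behavior for a hit reaction or stopping movement and disabling capsule collision at zero health.
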(event EventTick
  (params (DeltaSeconds :type Float%20%28single-precision%29))
  (bind _movespeed (Variables|Default|GetMoveSpeed))
  (bind _movement (Variables|Default|GetMovement))
  (bind _movement_2 (Variables|Default|GetMovement))
  (bind _paperflipbook (Variables|Default|GetPaperFlipbook))
  (bind _x (Math|Vector2D|BreakVector2D _movement_2))
  (bind (_x_2 _y) (Math|Vector2D|BreakVector2D _movement))
  (Variables|Default|SetAnimationResetTimer (- (Variables|Default|GetAnimationResetTimer) DeltaSeconds))
  (if (and (<= (Variables|Default|GetAnimationResetTimer) 0.0) (Variables|Default|GetIsActive))
    (CallFunction|UpdateState DeltaSeconds)
    (Transformation|AddActorWorldOffset (* (* (Math|Vector|MakeVector (Math|Float|Clamp(Float) _x_2 -1.0) 0.0 0.0) _movespeed) DeltaSeconds) true)
    (Transformation|AddActorWorldOffset (* (* (Math|Vector|MakeVector 0.0 (Math|Float|Clamp(Float) _y -1.0) 0.0) _movespeed) DeltaSeconds) true)
    (if (> _x 0.0)
      (Transformation|SetWorldRotation _paperflipbook "0, 0, 0" false false)
      (Variables|Default|SetFacingRight true)
      (CallFunction|SetAnimation "NewEnumerator1" :!label _label)
      (elif (< _x 0.0)
        (Transformation|SetWorldRotation _paperflipbook "0.000000,180.000000, 0" false false)
        (Variables|Default|SetFacingRight false)
        (goto _label)))))

(fn ConstructionScript)

(fn Damage
  (params (Amount :type Float%20%28single-precision%29) (Source :type Pawn%20Object%20Reference))
  (Variables|Default|SetTarget Source)
  (bind _output_get (Variables|Default|SetHealth (- (Variables|Default|GetHealth) Amount)))
  (if (<= _output_get 0.0)
    (CallFunction|SetState "NewEnumerator5")
    (CallFunction|SetAnimation "NewEnumerator3")
    (Variables|Default|SetMovement "")
    (Collision|SetCollisionEnabled (Variables|Default|GetCapsule) "NoCollision")
    (else
      (Variables|Default|SetAnimationResetTimer (Variables|Default|GetHitResetTime))
      (CallFunction|SetAnimation "NewEnumerator2")
      (CallFunction|SetState "NewEnumerator4"))))

(fn Activate
  (if (not (Variables|Default|GetIsActive))
    (Variables|Default|SetIsActive true)
    (CallFunction|SetState (Variables|Default|GetState))))

(fn UpdateState
  (params (Delta%20Time :type Float%20%28single-precision%29)))

(fn SetState
  (params (New%20State :type NPCStates%20Enum :default "NewEnumerator0")))

(fn SetAnimation
  (params (Animation :type NPCAnimations%20Enum :default "NewEnumerator0")))