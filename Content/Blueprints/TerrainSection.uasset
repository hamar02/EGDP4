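; Terrain section actor that forms a randomized piece of a 2D sprite level, with a building, a road and an enemy.
; The construction script picks random Paper2D sprites for the building and for child decals on building and road.
; Unless flagged first, BeginPlay spawns a random scaled-up enemy at its location, and SetFirst removes the StartBound component.
; Decal and enemy picks can index one past the array end, yielding nothing.
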(event EventBeginPlay
  (bind _enemies (Variables|Default|GetEnemies))
  (if (not (Variables|Default|GetIsFirst))
    (Game|SpawnActorfromClass (Utilities|Array|Get(acopy) _enemies (Math|Random|RandomIntegerinRange 0 (Utilities|Array|Length _enemies))) (Math|Transform|MakeTransform (Transformation|GetActorLocation) "0, 0, 0" "4.000000,4.000000,4.000000") "Undefined" 0 0)))

(fn ConstructionScript
  (bind _buildingsprites (Variables|Default|GetBuildingSprites))
  (bind _buildingdecals (Variables|Default|GetBuildingDecals))
  (bind _roaddecals (Variables|Default|GetRoadDecals))
  ;[1 1 1] Random building
  (Rendering|Components|Sprite|SetSprite (Variables|Default|GetPaperSpriteBuilding) (Utilities|Array|Get(acopy) _buildingsprites (Math|Random|RandomIntegerinRange 0 (- (Utilities|Array|Length _buildingsprites) 1))))
  ;[1 1 1] Random building decals
  (for _array_element (Components|GetChildrenComponents (Variables|Default|GetPaperSpriteBuilding) false)
    (bind _aspaper_sprite_component (Utilities|Casting|CastToPaperSpriteComponent _array_element))
    (Rendering|Components|Sprite|SetSprite _aspaper_sprite_component (Utilities|Array|Get(acopy) _buildingdecals (Math|Random|RandomIntegerinRange 0 (Utilities|Array|Length _buildingdecals)))))
  ;[1 1 1] Random road decals
  (for _array_element_2 (Components|GetChildrenComponents (Variables|Default|GetPaperSpriteRoad) false)
    (bind _aspaper_sprite_component_2 (Utilities|Casting|CastToPaperSpriteComponent _array_element_2))
    (Rendering|Components|Sprite|SetSprite _aspaper_sprite_component_2 (Utilities|Array|Get(acopy) _roaddecals (Math|Random|RandomIntegerinRange 0 (Utilities|Array|Length _roaddecals))))))

(fn SetFirst
  (params (SetFirst :type Boolean))
  (bind _output_get (Variables|Default|SetIsFirst SetFirst))
  (if (not _output_get)
    (Components|DestroyComponent (Variables|Default|GetStartBound))))