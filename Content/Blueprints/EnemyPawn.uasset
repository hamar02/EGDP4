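; Enemy pawn with Paper2D flipbook animation that hunts players and attacks players and civilians, extending a parent pawn's state and animation logic.
; While idle it sphere-traces for a player; becoming engaged alerts nearby enemies to the same target.
; Engaged, it steers toward the target on the XY plane, stopping in range to attack on a randomized timer.
; Attacks damage victims caught by a sphere trace on its facing side.
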(event EventTick
  (params (DeltaSeconds :type Float%20%28single-precision%29))
  (|CallParentFunction DeltaSeconds))

(event EventSetAnimation
  (params (Animation :type NPCAnimations%20Enum :default "NewEnumerator0"))
  (bind _paperflipbook (Variables|Default|GetPaperFlipbook))
  ;[1 1 1] Set Animation Override
  (switch Utilities|FlowControl|Switch|SwitchonNPCAnimations Animation
    (:NewEnumerator0
      (Sprite|SetFlipbook _paperflipbook))
    (:NewEnumerator1
      (Sprite|SetFlipbook _paperflipbook))
    (:NewEnumerator2
      (Sprite|SetFlipbook _paperflipbook))
    (:NewEnumerator3
      (Sprite|SetFlipbook _paperflipbook))
    (:NewEnumerator4
      (Sprite|SetFlipbook _paperflipbook))
    (:NewEnumerator5
      (Sprite|SetFlipbook _paperflipbook))))

(event EventSetState
  (params (New%20State :type NPCStates%20Enum :default "NewEnumerator0"))
  (bind _returnvalue (Transformation|GetActorLocation))
  ;[1 1 1] Set State Override
  (bind _output_get (Variables|Default|SetState New%20State))
  (switch Utilities|FlowControl|Switch|SwitchonNPCStates _output_get
    (:NewEnumerator4
      (bind _outhits (Collision|MultiSphereTraceForObjects _returnvalue _returnvalue (Variables|Default|GetAlertRange) (Utilities|Array|MakeArray "ObjectTypeQuery9") false 0 "None"))
      (for _array_element _outhits
        (bind _asenemy_pawn (Utilities|Casting|CastToEnemyPawn (.HitActor (Collision|BreakHitResult _array_element))))
        (CallFunction|Alert _asenemy_pawn (Variables|Default|GetTarget))))
    (:NewEnumerator7
      (CallFunction|SetAnimation "NewEnumerator5"))))

(event EventUpdateState
  (params (Delta%20Time :type Float%20%28single-precision%29))
  (bind _returnvalue (Transformation|GetActorLocation))
  (bind _returnvalue_2 (Transformation|GetActorLocation))
  (bind _attacktimerrange (Variables|Default|GetAttackTimerRange))
  (bind (_lowerbound _upperbound) (Utilities|Struct|BreakFloatRange _attacktimerrange))
  (bind (_x _y) (Math|Vector|BreakVector _returnvalue_2))
  ;[1 1 1] Update State Override
  (switch Utilities|FlowControl|Switch|SwitchonNPCStates (Variables|Default|GetState)
    (:NewEnumerator0
      (bind _outhits (Collision|MultiSphereTraceForObjects _returnvalue _returnvalue (Variables|Default|GetDetectionRange) (Utilities|Array|MakeArray "ObjectTypeQuery7") false 0 "None"))
      (for _array_element _outhits
        (bind _asplayer_pawn (Utilities|Casting|CastToPlayerPawn (.HitActor (Collision|BreakHitResult _array_element))))
        (Variables|Default|SetTarget _asplayer_pawn)
        (CallFunction|SetState "NewEnumerator4")))
    (:NewEnumerator4
      (Utilities|IsValid (Variables|Default|GetTarget)
        (:Is%20Valid
          (Variables|Default|SetMovement (Math|Vector2D|Normalize2D (- (Math|Vector2D|MakeVector2D (.X (Math|Vector|BreakVector (Transformation|GetActorLocation (Variables|Default|GetTarget)))) (.Y (Math|Vector|BreakVector (Transformation|GetActorLocation (Variables|Default|GetTarget))))) (Math|Vector2D|MakeVector2D _x _y))))
          (if (<= (Math|Vector2D|Vector2DLength (- (Math|Vector2D|MakeVector2D (.X (Math|Vector|BreakVector (Transformation|GetActorLocation (Variables|Default|GetTarget)))) (.Y (Math|Vector|BreakVector (Transformation|GetActorLocation (Variables|Default|GetTarget))))) (Math|Vector2D|MakeVector2D _x _y))) (Variables|Default|GetAttack%20Range))
            (bind _asplayer_pawn_2 (Utilities|Casting|CastToPlayerPawn (Variables|Default|GetTarget))
              (:then
                (if (not (Variables|/Game/Blueprints/PlayerPawn.PlayerPawn_C|GetIsDown _asplayer_pawn_2))
                  (Variables|Default|SetAttackTimer (- (Variables|Default|GetAttackTimer) Delta%20Time) :!label _label)
                  (Variables|Default|SetMovement "")
                  (CallFunction|SetAnimation "NewEnumerator0")
                  (if (<= (Variables|Default|GetAttackTimer) 0.0)
                    (CallFunction|Attack)
                    (Variables|Default|SetAttackTimer (Math|Random|RandomFloatinRange (.Value (Utilities|Struct|BreakFloatRangeBound _lowerbound)) (.Value (Utilities|Struct|BreakFloatRangeBound _upperbound)))))))
              (:CastFailed
                (goto _label)))))))))

(event EventBeginPlay
  (bind _attacktimerrange (Variables|Default|GetAttackTimerRange))
  (bind (_lowerbound _upperbound) (Utilities|Struct|BreakFloatRange _attacktimerrange))
  (Variables|Default|SetAttackTimer (Math|Random|RandomFloatinRange (.Value (Utilities|Struct|BreakFloatRangeBound _lowerbound)) (.Value (Utilities|Struct|BreakFloatRangeBound _upperbound)))))

(fn ConstructionScript
  (|CallParentFunction))

(fn Alert
  (params (Source :type Pawn%20Object%20Reference))
  (if (not (Utilities|Enum|Equal(Enum) (Variables|Default|GetState) "NewEnumerator5"))
    (Variables|Default|SetTarget Source)
    (CallFunction|SetState "NewEnumerator4")))

(fn Attack
  (bind _returnvalue (Transformation|GetActorLocation))
  (bind _facingright (Variables|Default|GetFacingRight))
  (bind _attack_range (Variables|Default|GetAttack%20Range))
  (bind _returnvalue_2 (* _attack_range 0.5))
  (bind _returnvalue_3 (* _returnvalue_2 -1.0))
  (bind _returnvalue_4 (select _facingright _returnvalue_2 _returnvalue_3))
  (bind _returnvalue_5 (Math|Vector|MakeVector _returnvalue_4 0.0 0.0))
  (bind _returnvalue_6 (+ _returnvalue _returnvalue_5))
  (CallFunction|SetAnimation "NewEnumerator4")
  (Variables|Default|SetAnimationResetTimer (Variables|Default|GetAttackResetTime))
  (bind _outhits (Collision|MultiSphereTraceForObjects _returnvalue_6 _returnvalue_6 _returnvalue_2 (Utilities|Array|MakeArray "ObjectTypeQuery7" "ObjectTypeQuery8") false 0 "None"))
  (for _array_element _outhits
    (bind _asplayer_pawn (Utilities|Casting|CastToPlayerPawn (.HitActor (Collision|BreakHitResult _array_element)))
      (:then
        (Default|Damage _asplayer_pawn (Variables|Default|GetFacingRight) (Variables|Default|GetAttack%20Damage)))
      (:CastFailed
        (bind _ascivilian_pawn (Utilities|Casting|CastToCivilianPawn (.HitActor (Collision|BreakHitResult _array_element))))
        (Default|Damage _ascivilian_pawn (Variables|Default|GetAttack%20Damage) self)))))