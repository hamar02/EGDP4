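; Balloon actor built on a Paper2D sprite that pops on Hit and then removes itself.
; Hit activates the particle system, swaps in the pop sprite and enables physics simulation on the sprite.
; Timed delays then stop the particles, hide the sprite and finally destroy the actor.
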(event Collision|EventHit
  (params (MyComp :type Primitive%20Component%20Object%20Reference) (Other :type Actor%20Object%20Reference) (OtherComp :type Primitive%20Component%20Object%20Reference) (bSelfMoved :type Boolean) (HitLocation :type Vector :default "0, 0, 0") (HitNormal :type Vector :default "0, 0, 0") (NormalImpulse :type Vector :default "0, 0, 0") (Hit :type Hit%20Result%20Structure%20%28by%20ref%29))
  (bind _papersprite (Variables|Default|GetPaperSprite))
  (Components|Activation|Activate (Variables|Default|GetParticleSystem) false)
  (Rendering|Components|Sprite|SetSprite _papersprite (Variables|Default|GetPopSprite))
  (Physics|SetSimulatePhysics (Variables|Default|GetPaperSprite) true)
  (Utilities|FlowControl|Delay 1.0)
  (Components|Activation|Deactivate (Variables|Default|GetParticleSystem))
  (Rendering|SetVisibility _papersprite false false)
  (Utilities|FlowControl|Delay 1.0)
  (Actor|DestroyActor))

(fn ConstructionScript)