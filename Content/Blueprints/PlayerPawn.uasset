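; Player pawn for a Paper2D beat 'em up with movement, melee attacks, directional blocking and knockdowns.
; Tick drives a camera clamped at the start X, wakes nearby NPCs and gates actions behind an animation timer.
; Hits dealt and taken shift Rage, amplified by a growing harmonic-sum multiplier, which scales attack damage.
; Full Rage overrides control, chaining high-damage leaps at the closest NPC until none is in range, then resets.
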(event EventBeginPlay
  (Variables|Default|SetCameraMinX (.X (Math|Vector|BreakVector (Transformation|GetActorLocation))))
  (bind _outactors (Actor|GetAllActorsOfClass "/Script/Engine.CameraActor"))
  (for _array_element _outactors
    (if (Utilities|Enum|Equal(Enum) (Utilities|GetObjectName _array_element) "PlayerCamera")
      (Variables|Default|SetCamera _array_element)))
  (bind _outactors_2 (Actor|GetAllActorsOfClass "/Game/Blueprints/NPCPawn.NPCPawn_C"))
  (Variables|Default|SetNPCs _outactors_2))

(event EventTick
  (params (DeltaSeconds :type Float%20%28single-precision%29))
  (bind _movespeed (Variables|Default|GetMoveSpeed))
  (bind _blockinput (Variables|Default|GetBlockInput))
  (bind _movement (Variables|Default|GetMovement))
  (bind _camera (Variables|Default|GetCamera))
  (bind _movement_2 (Variables|Default|GetMovement))
  (bind _paperflipbook (Variables|Default|GetPaperFlipbook))
  (bind (_x _y) (Math|Vector2D|BreakVector2D _movement_2))
  (bind _returnvalue (Transformation|GetActorLocation _camera))
  (bind (_x_2 _y_2) (Math|Vector2D|BreakVector2D _movement))
  (bind (_x_3 _y_3 _z) (Math|Vector|BreakVector _returnvalue))
  (CallFunction|ActivateNPCs)
  (Transformation|SetActorLocation _camera (Math|Vector|MakeVector (Math|Float|Max(Float) (.X (Math|Vector|BreakVector (Transformation|GetActorLocation))) (Variables|Default|GetCameraMinX)) _y_3 _z) false false)
  (if (Variables|Default|GetIsLeaping)
    (CallFunction|LeapUpdate DeltaSeconds)
    (elif (< (Variables|Default|GetRage) 1.0)
      (bind _output_get (Variables|Default|SetAnimResetTimer (- (Variables|Default|GetAnimResetTimer) DeltaSeconds)))
      (if (and (Variables|Default|GetIsBlocking) _blockinput)
        (CallFunction|Block :!label _label)
        (elif (<= _output_get 0.0)
          (if _blockinput
            (goto _label)
            (else
              (Variables|Default|SetIsDown false)
              (Transformation|AddActorWorldOffset (* (* (Math|Vector|MakeVector (Math|Float|Clamp(Float) _x_2 -1.0) 0.0 0.0) _movespeed) DeltaSeconds) true)
              (Transformation|AddActorWorldOffset (* (* (Math|Vector|MakeVector 0.0 (Math|Float|Clamp(Float) _y_2 -1.0) 0.0) _movespeed) DeltaSeconds) true)
              (if (> _x 0.0)
                (Transformation|SetWorldRotation _paperflipbook "0, 0, 0" false false)
                (Variables|Default|SetFacingRight true)
                (CallFunction|SetAnimation :!label _label_2)
                (elif (< _x 0.0)
                  (Transformation|SetWorldRotation _paperflipbook "0.000000,180.000000, 0" false false)
                  (Variables|Default|SetFacingRight false)
                  (goto _label_2)
                  (elif (!= _y 0.0)
                    (CallFunction|SetAnimation)
                    (else
                      (CallFunction|SetAnimation)))))))))
      (else
        (CallFunction|RageAttack)))))

(event Input|ActionEvents|InputActionAttack
  (params (Key :type Key%20Structure))
  (:Pressed
    (if (<= (Variables|Default|GetAnimResetTimer) 0.0)
      (CallFunction|Attack))))

(event Input|ActionEvents|InputActionBlock
  (params (Key :type Key%20Structure))
  (:Pressed
    (Variables|Default|SetBlockInput true))
  (:Released
    (Variables|Default|SetBlockInput false)))

(event Input|AxisEvents|InputAxisMoveRight
  (params (AxisValue :type Float%20%28single-precision%29))
  (Variables|Default|SetMovement (Math|Vector2D|MakeVector2D AxisValue (.Y (Math|Vector2D|BreakVector2D (Variables|Default|GetMovement))))))

(event Input|AxisEvents|InputAxisMoveUp
  (params (AxisValue :type Float%20%28single-precision%29))
  (Variables|Default|SetMovement (Math|Vector2D|MakeVector2D (.X (Math|Vector2D|BreakVector2D (Variables|Default|GetMovement))) AxisValue)))

(fn ConstructionScript)

(fn Attack
  (bind _returnvalue (Transformation|GetActorLocation))
  (bind _attackrange (Variables|Default|GetAttackRange))
  (bind _facingright (Variables|Default|GetFacingRight))
  (bind _returnvalue_2 (* _attackrange 0.5))
  (bind _returnvalue_3 (* _returnvalue_2 -1.0))
  (bind _returnvalue_4 (select _facingright _returnvalue_2 _returnvalue_3))
  (bind _returnvalue_5 (Math|Vector|MakeVector _returnvalue_4 0.0 0.0))
  (bind _returnvalue_6 (+ _returnvalue _returnvalue_5))
  (CallFunction|SetAnimation)
  (CallFunction|SetAnimation)
  (Variables|Default|SetAnimResetTimer (Variables|Default|GetAttackResetTime))
  (bind _outhits (Collision|MultiSphereTraceForObjects _returnvalue_6 _returnvalue_6 _returnvalue_2 (Utilities|Array|MakeArray "ObjectTypeQuery9" "ObjectTypeQuery8") false 0 "None"))
  (for _array_element _outhits
    (bind _asnpcpawn (Utilities|Casting|CastToNPCPawn (.HitActor (Collision|BreakHitResult _array_element))))
    (Default|Damage _asnpcpawn (Math|Float|Lerp (Variables|Default|GetMinDamage) (Variables|Default|GetMaxDamage) (Math|Float|MapRangeClamped (Variables|Default|GetRage) -1.0 1.0 0.0 1.0)) self)
    (CallFunction|AddRage 0.05 0.2)))

(fn SetAnimation
  (params (Animation :type Paper%20Flipbook%20Object%20Reference))
  (Sprite|SetFlipbook (Variables|Default|GetPaperFlipbook) Animation))

(fn Block
  (if (or (<= (Variables|Default|GetAnimResetTimer) 0.0) (Variables|Default|GetIsBlocking))
    (Variables|Default|SetIsBlocking true)
    (CallFunction|SetAnimation)
    (Variables|Default|SetAnimResetTimer (Variables|Default|GetBlockResetTime))))

(fn Damage
  (params (RightDirection :type Boolean) (Damage :type Float%20%28single-precision%29))
  (if (not (Variables|Default|GetIsDown))
    (if (and (Variables|Default|GetIsBlocking) (Math|Boolean|NotEqual(Boolean) (Variables|Default|GetFacingRight) RightDirection))
      (CallFunction|AddRage -0.05 0.0)
      (else
        (bind _output_get (Variables|Default|SetHealth (- (Variables|Default|GetHealth) Damage)))
        (if (<= _output_get 0.0)
          (Variables|Default|SetAnimResetTimer (Variables|Default|GetKnockoutResetTime))
          (CallFunction|SetAnimation)
          (CallFunction|AddRage -0.6 1.0)
          (Variables|Default|SetHealth 1.0)
          (Variables|Default|SetIsDown true)
          (else
            (Variables|Default|SetAnimResetTimer (Variables|Default|GetDamageResetTime))
            (CallFunction|SetAnimation)
            (CallFunction|AddRage -0.3 0.3)))))))

(fn AddRage
  (params (Amount :type Float%20%28single-precision%29) (MultIncrease :type Float%20%28single-precision%29))
  (bind _output_get (Variables|Default|SetRageMultiplier (+ MultIncrease (Variables|Default|GetRageMultiplier))))
  (for _index (range 1 (Math|Float|Truncate _output_get))
    (bind _output_get_2 (LocalVariables|SetAcc (+ (LocalVariables|GetAcc) (/ 1.0 (Math|Conversions|ToFloat(Integer) _index)))))
    (Variables|Default|SetRage (Math|Float|Clamp(Float) (+ (Variables|Default|GetRage) (* Amount (Math|Float|Lerp _output_get_2 (+ _output_get_2 (/ 1.0 (Math|Conversions|ToFloat(Integer) (+ (Math|Float|Truncate _output_get) 1)))) (- _output_get (Math|Conversions|ToFloat(Integer) (Math|Float|Truncate _output_get)))))) -1.0))))

(fn ActivateNPCs
  (for (_array_element _array_index) (Variables|Default|GetNPCs)
    (if (Utilities|IsValid _array_element)
      (if (<= (Math|Float|Absolute(Float) (- (.X (Math|Vector|BreakVector (Transformation|GetActorLocation _array_element))) (.X (Math|Vector|BreakVector (Transformation|GetActorLocation))))) (Variables|Default|GetActivationRange))
        (Default|Activate _array_element))
      (else
        (Utilities|Array|RemoveIndex (Variables|Default|GetNPCs) _array_index)))))

(fn RageAttack
  (bind _returnvalue (Transformation|GetActorLocation))
  (bind _returnvalue_2 (Transformation|GetActorLocation))
  (bind (_outhits _returnvalue_3) (Collision|MultiSphereTraceForObjects _returnvalue_2 _returnvalue_2 (Variables|Default|GetRageAttackRange) (Utilities|Array|MakeArray "ObjectTypeQuery9") false 0 "None"))
  (if _returnvalue_3
    (for (_array_element _array_index) _outhits
      (if (!= _array_index 0)
        (if (< (Math|Vector|VectorLength (- (Transformation|GetActorLocation) (Transformation|GetActorLocation (.HitActor (Collision|BreakHitResult _array_element))))) (LocalVariables|GetClosestDistance))
          (LocalVariables|SetClosestIndex _array_index)
          (LocalVariables|SetClosestDistance (Math|Vector|VectorLength (- (Transformation|GetActorLocation) (Transformation|GetActorLocation (.HitActor (Collision|BreakHitResult _array_element))))) :!label _label))
        (else
          (goto _label))))
    (bind _asnpcpawn (Utilities|Casting|CastToNPCPawn (.HitActor (Collision|BreakHitResult (Utilities|Array|Get(acopy) _outhits (LocalVariables|GetClosestIndex))))))
    (CallFunction|Leap _asnpcpawn)
    (else
      (bind (_outhits_2 _returnvalue_4) (Collision|MultiSphereTraceForObjects _returnvalue _returnvalue (Variables|Default|GetRageAttackRange) (Utilities|Array|MakeArray "ObjectTypeQuery8") false 0 "None"))
      (if _returnvalue_4
        (for (_array_element_2 _array_index_2) _outhits_2
          (if (!= _array_index_2 0)
            (if (< (Math|Vector|VectorLength (- (Transformation|GetActorLocation) (Transformation|GetActorLocation (.HitActor (Collision|BreakHitResult _array_element_2))))) (LocalVariables|GetClosestDistance))
              (LocalVariables|SetClosestIndex _array_index_2)
              (LocalVariables|SetClosestDistance (Math|Vector|VectorLength (- (Transformation|GetActorLocation) (Transformation|GetActorLocation (.HitActor (Collision|BreakHitResult _array_element_2))))) :!label _label_2))
            (else
              (goto _label_2))))
        (bind _asnpcpawn_2 (Utilities|Casting|CastToNPCPawn (.HitActor (Collision|BreakHitResult (Utilities|Array|Get(acopy) _outhits_2 (LocalVariables|GetClosestIndex))))))
        (CallFunction|Leap _asnpcpawn_2)
        (else
          (Variables|Default|SetAnimResetTimer (Variables|Default|GetRageResetTime))
          (Sprite|SetFlipbook (Variables|Default|GetPaperFlipbook))
          (Variables|Default|SetRage 0.0))))))

(fn Leap
  (params (Victim :type NPC%20Pawn%20Object%20Reference))
  (Sprite|SetFlipbook (Variables|Default|GetPaperFlipbook))
  (Variables|Default|SetIsLeaping true)
  (Variables|Default|SetTarget Victim)
  (Variables|Default|SetLeapTimer (Variables|Default|GetLeapCooldown)))

(fn LeapUpdate
  (params (Delta%20Time :type Float%20%28single-precision%29))
  (bind _returnvalue (Transformation|GetActorLocation))
  (bind _returnvalue_2 (Transformation|GetActorLocation))
  (bind (_x _y) (Math|Vector|BreakVector _returnvalue))
  (bind (_x_2 _y_2) (Math|Vector|BreakVector _returnvalue_2))
  (bind _output_get (Variables|Default|SetLeapTimer (- (Variables|Default|GetLeapTimer) Delta%20Time)))
  (if (<= _output_get 0.0)
    (Collision|SetCollisionEnabled (Variables|Default|GetCapsule) "NoCollision")
    (Transformation|AddActorWorldOffset (* (* (Math|Vector|MakeVector (Math|Float|Clamp(Float) (.X (Math|Vector2D|BreakVector2D (Math|Vector2D|Normalize2D (- (Math|Vector2D|MakeVector2D (.X (Math|Vector|BreakVector (Transformation|GetActorLocation (Variables|Default|GetTarget)))) (.Y (Math|Vector|BreakVector (Transformation|GetActorLocation (Variables|Default|GetTarget))))) (Math|Vector2D|MakeVector2D _x_2 _y_2))))) -1.0) 0.0 0.0) 1e+03) Delta%20Time))
    (Transformation|AddActorWorldOffset (* (* (Math|Vector|MakeVector 0.0 (Math|Float|Clamp(Float) (.Y (Math|Vector2D|BreakVector2D (Math|Vector2D|Normalize2D (- (Math|Vector2D|MakeVector2D (.X (Math|Vector|BreakVector (Transformation|GetActorLocation (Variables|Default|GetTarget)))) (.Y (Math|Vector|BreakVector (Transformation|GetActorLocation (Variables|Default|GetTarget))))) (Math|Vector2D|MakeVector2D _x_2 _y_2))))) -1.0) 0.0) 1e+03) Delta%20Time))
    (Transformation|SetWorldRotation (Variables|Default|GetPaperFlipbook) (Math|Rotator|MakeRotator 0.0 0.0 (select (>= (.X (Math|Vector2D|BreakVector2D (Math|Vector2D|Normalize2D (- (Math|Vector2D|MakeVector2D (.X (Math|Vector|BreakVector (Transformation|GetActorLocation (Variables|Default|GetTarget)))) (.Y (Math|Vector|BreakVector (Transformation|GetActorLocation (Variables|Default|GetTarget))))) (Math|Vector2D|MakeVector2D _x_2 _y_2))))) 0.0) 0.0 1.8e+02)) false false)
    (if (<= (Math|Vector2D|Vector2DLength (- (Math|Vector2D|MakeVector2D (.X (Math|Vector|BreakVector (Transformation|GetActorLocation (Variables|Default|GetTarget)))) (.Y (Math|Vector|BreakVector (Transformation|GetActorLocation (Variables|Default|GetTarget))))) (Math|Vector2D|MakeVector2D _x _y))) 25.0)
      (Collision|SetCollisionEnabled (Variables|Default|GetCapsule) "QueryAndPhysics")
      (Default|Damage (Variables|Default|GetTarget) 1e+03 self)
      (Variables|Default|SetIsLeaping false)
      (Variables|Default|SetTarget 0))))