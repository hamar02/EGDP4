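; CivilianPawn is a Paper2D civilian character that wanders and flees from its target when engaged, overriding state and animation events from a parent pawn.
; UpdateState picks a random left or right Movement when Wandering with no X movement, or a normalized XY direction away from a valid Target when Engaged.
; SetState stores the new state, and SetAnimation switches on Idle, Walk, Hit and Down to set the flipbook.
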(event EventTick
  (params (DeltaSeconds :type Float%20%28single-precision%29))
  (|CallParentFunction DeltaSeconds))

(event EventUpdateState
  (params (Delta%20Time :type Float%20%28single-precision%29))
  (bind _returnvalue (Transformation|GetActorLocation))
  (bind _target (Variables|Default|GetTarget))
  (bind _returnvalue_2 (Transformation|GetActorLocation _target))
  (bind (_x _y) (Math|Vector|BreakVector _returnvalue))
  (bind (_x_2 _y_2) (Math|Vector|BreakVector _returnvalue_2))
  ;[1 1 1] Update State Override
  (switch Utilities|FlowControl|Switch|SwitchonNPCStates (Variables|Default|GetState)
    (:NewEnumerator6
      (if (== (.X (Math|Vector2D|BreakVector2D (Variables|Default|GetMovement))) 0.0)
        (Variables|Default|SetMovement (Utilities|Select :Index (Math|Random|RandomInteger 1) :Option%200 "(X=1.000000,Y=0.000000)" :Option%201 "(X=-1.000000,Y=0.000000)"))))
    (:NewEnumerator4
      (Utilities|IsValid _target
        (:Is%20Valid
          (Variables|Default|SetMovement (Math|Vector2D|Normalize2D (- (Math|Vector2D|MakeVector2D _x _y) (Math|Vector2D|MakeVector2D _x_2 _y_2)))))))))

(event EventSetState
  (params (New%20State :type NPCStates%20Enum :default "NewEnumerator0"))
  ;[1 1 1] Set State Override
  (Variables|Default|SetState New%20State))

(event EventSetAnimation
  (params (Animation :type NPCAnimations%20Enum :default "NewEnumerator0"))
  (bind _paperflipbook (Variables|Default|GetPaperFlipbook))
  ;[1 1 1] Set Animation Override
  (switch Utilities|FlowControl|Switch|SwitchonNPCAnimations Animation
    (:NewEnumerator0
      (Sprite|SetFlipbook _paperflipbook))
    (:NewEnumerator1
      (Sprite|SetFlipbook _paperflipbook))
    (:NewEnumerator2
      (Sprite|SetFlipbook _paperflipbook))
    (:NewEnumerator3
      (Sprite|SetFlipbook _paperflipbook))))

(fn ConstructionScript
  (|CallParentFunction))