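; Damageable physics object for a 2D side-scroller that registers its value with the game mode and hides its widget after five seconds.
; Point damage, or hits where both actors move fast enough, call Take Damage, which applies an impulse and lowers the value.
; While the value stays above -1, damage flashes particles, reports the fixed loss to the game mode, then destroys the actor if depleted.
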(event EventBeginPlay
  (bind _as2dside_scroller_game_mode (Utilities|Casting|CastTo2DSideScrollerGameMode (Game|GetGameMode)))
  (Default|SetupValue _as2dside_scroller_game_mode (Variables|Default|GetValue$))
  (Variables|Default|SetCurrentValue$ (Variables|Default|GetValue$))
  (Utilities|FlowControl|Delay 5.0)
  (Rendering|SetVisibility (Variables|Default|GetWidget) false false))

(event Collision|EventHit
  (params (MyComp :type Primitive%20Component%20Object%20Reference) (Other :type Actor%20Object%20Reference) (OtherComp :type Primitive%20Component%20Object%20Reference) (bSelfMoved :type Boolean) (HitLocation :type Vector :default "0, 0, 0") (HitNormal :type Vector :default "0, 0, 0") (NormalImpulse :type Vector :default "0, 0, 0") (Hit :type Hit%20Result%20Structure%20%28by%20ref%29))
  (bind _returnvalue (Transformation|GetVelocity Other))
  (bind _returnvalue_2 (Transformation|GetVelocity))
  (bind _velocitybeforedamagetaken (Variables|Default|GetVelocityBeforeDamageTaken))
  (bind _returnvalue_3 (Math|Vector|VectorLength _returnvalue))
  (bind _returnvalue_4 (Math|Vector|VectorLength _returnvalue_2))
  (if (not (or (< _returnvalue_3 _velocitybeforedamagetaken) (< _returnvalue_4 _velocitybeforedamagetaken)))
    (Utilities|TakeDamage HitNormal (+ _returnvalue_3 _returnvalue_4))))

(event Game|Damage|EventPointDamage
  (params (Damage :type Float%20%28single-precision%29) (DamageType :type Damage%20Type%20Object%20Reference) (HitLocation :type Vector :default "0, 0, 0") (HitNormal :type Vector :default "0, 0, 0") (HitComponent :type Primitive%20Component%20Object%20Reference) (BoneName :type Name :default "None") (ShotFromDirection :type Vector :default "0, 0, 0") (InstigatedBy :type Controller%20Object%20Reference) (DamageCauser :type Actor%20Object%20Reference) (HitInfo :type Hit%20Result%20Structure%20%28by%20ref%29))
  (Utilities|TakeDamage ShotFromDirection Damage))

(fn ConstructionScript)